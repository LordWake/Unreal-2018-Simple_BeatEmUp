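; BP_MyPlayer is the player Blueprint, handling melee hits on enemies and destructibles.
; On BeginPlay it assigns its two hit boxes and two knives to variables; on Tick it fixes the camera controller's rotation while the player is dead.
; Box overlaps deal light punch damage with camera shake and random sounds, while HardBox overlaps deal heavier knife damage to BP_MyEnemy and BP_Kentucky.
; Both boxes fracture destructibles through line-traced radial damage.
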(event OnComponentBeginOverlap(Box)
  (params (OverlappedComponent :type Primitive%20Component%20Object%20Reference) (OtherActor :type Actor%20Object%20Reference) (OtherComp :type Primitive%20Component%20Object%20Reference) (OtherBodyIndex :type Integer) (bFromSweep :type Boolean) (SweepResult :type Hit%20Result%20Structure%20%28by%20ref%29))
  (bind _returnvalue (Transformation|GetActorLocation))
  (bind _returnvalue_2 (Transformation|GetActorLocation))
  (Utilities|FlowControl|Sequence
    (:then_0
      ;[1 1 1] DestructibleActor
      (if (!= (Actor|GetComponentbyClass OtherActor "/Script/ApexDestruction.DestructibleComponent") 0)
        (bind _outhit (Collision|LineTraceByChannel (Transformation|GetActorLocation) (Transformation|GetActorLocation OtherActor) "TraceTypeQuery1" false 0 "None"))
        (Game|Damage|ApplyRadialDamage 5e+01 (.Location (Collision|BreakHitResult _outhit)) 2.0 0 0 0 0 false "ECC_Visibility")))
    (:then_1
      (bind _asbp_my_enemy (Utilities|Casting|CastToBP_MyEnemy OtherActor))
      (Class|MyEnemy|TakeDamage _asbp_my_enemy 5.0)
      (Camera|PlayWorldCameraShake "/Game/Blueprints/Actors/Player/BP_MyCameraShake.BP_MyCameraShake_C" (Transformation|GetActorLocation) 0.0 2.5e+02)
      (if (<= (Math|Random|RandomFloatinRange 0.0 5e+01) 25.0)
        (Audio|PlaySoundatLocation "/Game/SoundsFX/Player/PlayerPunch1.PlayerPunch1" _returnvalue "0, 0, 0" 1.0 1.0 0.0 0 0 0)
        (elif (<= (Math|Random|RandomFloatinRange 0.0 5e+01) 25.0)
          (Audio|PlaySoundatLocation "/Game/SoundsFX/Player/PlayerPunch2.PlayerPunch2" _returnvalue "0, 0, 0" 1.0 1.0 0.0 0 0 0)
          (else
            (Audio|PlaySoundatLocation "/Game/SoundsFX/Player/PlayerPunch3.PlayerPunch3" _returnvalue "0, 0, 0" 1.0 1.0 0.0 0 0 0)))))
    (:then_2
      (bind _asbp_kentucky (Utilities|Casting|CastToBP_Kentucky OtherActor))
      (Class|Kentucky|TakeDamage _asbp_kentucky 5.0)
      (Camera|PlayWorldCameraShake "/Game/Blueprints/Actors/Player/BP_MyCameraShake.BP_MyCameraShake_C" (Transformation|GetActorLocation) 0.0 2.5e+02)
      (if (<= (Math|Random|RandomFloatinRange 0.0 5e+01) 25.0)
        (Audio|PlaySoundatLocation "/Game/SoundsFX/Player/PlayerPunch1.PlayerPunch1" _returnvalue_2 "0, 0, 0" 1.0 1.0 0.0 0 0 0)
        (elif (<= (Math|Random|RandomFloatinRange 0.0 5e+01) 25.0)
          (Audio|PlaySoundatLocation "/Game/SoundsFX/Player/PlayerPunch2.PlayerPunch2" _returnvalue_2 "0, 0, 0" 1.0 1.0 0.0 0 0 0)
          (else
            (Audio|PlaySoundatLocation "/Game/SoundsFX/Player/PlayerPunch3.PlayerPunch3" _returnvalue_2 "0, 0, 0" 1.0 1.0 0.0 0 0 0)))))))

(event OnComponentBeginOverlap(HardBox)
  (params (OverlappedComponent :type Primitive%20Component%20Object%20Reference) (OtherActor :type Actor%20Object%20Reference) (OtherComp :type Primitive%20Component%20Object%20Reference) (OtherBodyIndex :type Integer) (bFromSweep :type Boolean) (SweepResult :type Hit%20Result%20Structure%20%28by%20ref%29))
  (Utilities|FlowControl|Sequence
    (:then_0
      ;[1 1 1] DestructibleActor
      (if (!= (Actor|GetComponentbyClass OtherActor "/Script/ApexDestruction.DestructibleComponent") 0)
        (bind _outhit (Collision|LineTraceByChannel (Transformation|GetActorLocation) (Transformation|GetActorLocation OtherActor) "TraceTypeQuery1" false 0 "None"))
        (Game|Damage|ApplyRadialDamage 5e+01 (.Location (Collision|BreakHitResult _outhit)) 2.0 0 0 0 0 false "ECC_Visibility")))
    (:then_1
      (bind _asbp_my_enemy (Utilities|Casting|CastToBP_MyEnemy OtherActor))
      (Class|MyEnemy|TakeDamage _asbp_my_enemy 1e+01)
      (Audio|PlaySoundatLocation "/Game/SoundsFX/Player/Player_Knife.Player_Knife" (Transformation|GetActorLocation) "0, 0, 0" 1.0 1.0 0.0 0 0 0))
    (:then_2
      (bind _asbp_kentucky (Utilities|Casting|CastToBP_Kentucky OtherActor))
      (Class|Kentucky|TakeDamage _asbp_kentucky 1e+01)
      (Audio|PlaySoundatLocation "/Game/SoundsFX/Player/Player_Knife.Player_Knife" (Transformation|GetActorLocation) "0, 0, 0" 1.0 1.0 0.0 0 0 0))))

(event EventBeginPlay
  (Utilities|FlowControl|Sequence
    (:then_0
      (Variables|Default|SetboxTrigger (Variables|Default|GetBox)))
    (:then_1
      (Variables|Default|SethardBoxTrigger (Variables|Default|GetHardBox)))
    (:then_2
      (Variables|Default|SetmyKnife (Variables|Default|GetKnife)))
    (:then_3
      (Variables|Default|SetmySecondKnife (Variables|Default|GetSecondKnife)))))

(event EventTick
  (params (DeltaSeconds :type Float%20%28single-precision%29))
  (if (Variables|Default|GetplayerIsDead)
    (Transformation|SetRelativeRotation (Variables|Default|GetCameraController) "300.000000, 0, 0" false false)))

(fn ConstructionScript)