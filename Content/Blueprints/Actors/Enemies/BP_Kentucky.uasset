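; BP_Kentucky is an enemy actor that deals melee punch damage to BP_MyPlayer.
; Normal and hard trigger overlaps call the player's DamageEvent, the hard one for double damage, and play one of two random punch sounds.
; BeginPlay stores both triggers in variables, and Tick updates the distance to the player.
; RadiusCheck forwards begin overlaps to MyBeginOverlap, while the logic clearing ClosestObstacle is disconnected.
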(event OnComponentBeginOverlap(NormalTrigger)
  (params (OverlappedComponent :type Primitive%20Component%20Object%20Reference) (OtherActor :type Actor%20Object%20Reference) (OtherComp :type Primitive%20Component%20Object%20Reference) (OtherBodyIndex :type Integer) (bFromSweep :type Boolean) (SweepResult :type Hit%20Result%20Structure%20%28by%20ref%29))
  (bind _returnvalue (Transformation|GetActorLocation))
  (bind _asbp_my_player (Utilities|Casting|CastToBP_MyPlayer OtherActor))
  (Class|MyPlayer|DamageEvent _asbp_my_player 2.5)
  (if (<= (Math|Random|RandomFloatinRange 0.0 5e+01) 25.0)
    (Audio|PlaySoundatLocation "/Game/SoundsFX/Enemy/EnemyPunch1.EnemyPunch1" _returnvalue "0, 0, 0" 1.0 1.0 0.0 0 0 0)
    (else
      (Audio|PlaySoundatLocation "/Game/SoundsFX/Enemy/EnemyPunch2.EnemyPunch2" _returnvalue "0, 0, 0" 1.0 1.0 0.0 0 0 0))))

(event OnComponentBeginOverlap(HardTrigger)
  (params (OverlappedComponent :type Primitive%20Component%20Object%20Reference) (OtherActor :type Actor%20Object%20Reference) (OtherComp :type Primitive%20Component%20Object%20Reference) (OtherBodyIndex :type Integer) (bFromSweep :type Boolean) (SweepResult :type Hit%20Result%20Structure%20%28by%20ref%29))
  (bind _returnvalue (Transformation|GetActorLocation))
  (bind _asbp_my_player (Utilities|Casting|CastToBP_MyPlayer OtherActor))
  (Class|MyPlayer|DamageEvent _asbp_my_player 5.0)
  (if (<= (Math|Random|RandomFloatinRange 0.0 5e+01) 25.0)
    (Audio|PlaySoundatLocation "/Game/SoundsFX/Enemy/EnemyPunch1.EnemyPunch1" _returnvalue "0, 0, 0" 1.0 1.0 0.0 0 0 0)
    (else
      (Audio|PlaySoundatLocation "/Game/SoundsFX/Enemy/EnemyPunch2.EnemyPunch2" _returnvalue "0, 0, 0" 1.0 1.0 0.0 0 0 0))))

(event OnComponentBeginOverlap(RadiusCheck)
  (params (OverlappedComponent :type Primitive%20Component%20Object%20Reference) (OtherActor :type Actor%20Object%20Reference) (OtherComp :type Primitive%20Component%20Object%20Reference) (OtherBodyIndex :type Integer) (bFromSweep :type Boolean) (SweepResult :type Hit%20Result%20Structure%20%28by%20ref%29))
  (Class|Kentucky|MyBeginOverlap OtherActor))

(event OnComponentEndOverlap(RadiusCheck)
  (params (OverlappedComponent :type Primitive%20Component%20Object%20Reference) (OtherActor :type Actor%20Object%20Reference) (OtherComp :type Primitive%20Component%20Object%20Reference) (OtherBodyIndex :type Integer)))

(event EventBeginPlay
  (Utilities|FlowControl|Sequence
    (:then_0
      (Variables|Default|SetnormalBoxTrigger (Variables|Default|GetNormalTrigger)))
    (:then_1
      (Variables|Default|SethardBoxTrigger (Variables|Default|GetHardTrigger)))))

(event EventTick
  (params (DeltaSeconds :type Float%20%28single-precision%29))
  (Variables|Default|SetdistanceToPlayer (Transformation|GetDistanceTo (Game|GetPlayerCharacter 0))))

(fn ConstructionScript)